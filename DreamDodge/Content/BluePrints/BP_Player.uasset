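; Player Blueprint that turns Enhanced Input actions into movement, jumping, dimension swapping and dodge meter use.
; On BeginPlay it adds the input mapping context to its player controller, then calls Setup.
; A/D feed opposite directions into MoveInput, W and Space share JumpInput, and E swaps dimensions.
; Left mouse start and completion both call UseDodgeMeterValue with elapsed time, while cancel clears the StartedHealing flag.
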(event `self.ReceiveBeginPlay`
  (bind _asplayer_controller (cast `PlayerController` (`self.GetController`)))
  (`EnhancedInputSubsystemInterface.AddMappingContext` (pcsubsystem `EnhancedInputLocalPlayerSubsystem` _asplayer_controller) "/Game/Input/InputMap.InputMap" 0 (struct))
  (`self.Setup`))

(event `EnhancedInput|/Game/Input/IA_A`
  (params (ActionValue :type Boolean) (ElapsedSeconds :type "Float (double-precision)") (TriggeredSeconds :type "Float (double-precision)") (InputAction :type "InputAction Object Reference" :default "/Game/Input/IA_A.IA_A"))
  (:`Triggered`
    (`self.MoveInput` 1)))

(event `EnhancedInput|/Game/Input/IA_E`
  (params (ActionValue :type Boolean) (ElapsedSeconds :type "Float (double-precision)") (TriggeredSeconds :type "Float (double-precision)") (InputAction :type "InputAction Object Reference" :default "/Game/Input/IA_E.IA_E"))
  (:`Triggered`
    (`self.SwapDimensions`)))

(event `EnhancedInput|/Game/Input/IA_W`
  (params (ActionValue :type Boolean) (ElapsedSeconds :type "Float (double-precision)") (TriggeredSeconds :type "Float (double-precision)") (InputAction :type "InputAction Object Reference" :default "/Game/Input/IA_W.IA_W"))
  (:`Triggered`
    (`self.JumpInput` :!label _label)))

(event `EnhancedInput|/Game/Input/IA_D`
  (params (ActionValue :type Boolean) (ElapsedSeconds :type "Float (double-precision)") (TriggeredSeconds :type "Float (double-precision)") (InputAction :type "InputAction Object Reference" :default "/Game/Input/IA_D.IA_D"))
  (:`Triggered`
    (`self.MoveInput` -1)))

(event `EnhancedInput|/Game/Input/IA_Space`
  (params (ActionValue :type Boolean) (ElapsedSeconds :type "Float (double-precision)") (TriggeredSeconds :type "Float (double-precision)") (InputAction :type "InputAction Object Reference" :default "/Game/Input/IA_Space.IA_Space"))
  (:`Triggered`
    (goto _label)))

(event `EnhancedInput|/Game/Input/IA_LMB`
  (params (ActionValue :type Boolean) (ElapsedSeconds :type "Float (double-precision)") (TriggeredSeconds :type "Float (double-precision)") (InputAction :type "InputAction Object Reference" :default "/Game/Input/IA_LMB.IA_LMB"))
  (:`Started`
    (`self.UseDodgeMeterValue` ElapsedSeconds :!label _label_2))
  (:`Canceled`
    (set `self.StartedHealing` false))
  (:`Completed`
    (goto _label_2)))

(fn `UserConstructionScript`
  (`parent.UserConstructionScript`))